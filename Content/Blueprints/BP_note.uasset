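; BP_note is a rhythm-game block or bomb, placed by time, line and layer, with a cut direction.
; UpdateNote, run from the construction script, picks meshes and materials from Type, including a special lightning-bolt variant, then calls UpdateTransform.
; UpdateTransform rotates the mesh by Direction, offsets it on a 4x3 grid and moves the actor along Y by Time.
; FixValues wraps Line and Layer into range, and GetProperties packs the note into a struct.
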(event `Update Note`
  (bind _mesh (`self.Mesh`))
  (bind _arrow (`self.Arrow`))
  (bind _arrow_2 (`self.Arrow`))
  (bind _mesh_2 (`self.Mesh`))
  (bind _mesh_3 (`self.Mesh`))
  (bind _arrow_3 (`self.Arrow`))
  (`self.FixValues`)
  (`|ExecutionSequence`
    (:`then_0`
      (switch `int` (`self.Type`)
        (:`Default`
          ;[1 1 1] Tobii
          (if (== (`self.Type`) 42)
            (`StaticMeshComponent.SetStaticMesh` _mesh_2 "/Game/Meshes/SM_CubeNote.SM_CubeNote")
            (`PrimitiveComponent.SetMaterial` _mesh_2 0 "/Game/Materials/M_CubeNote_mag.M_CubeNote_mag")
            (`PrimitiveComponent.SetMaterial` _arrow 0 "/Game/Materials/M_Arrow_mag.M_Arrow_mag")
            (`StaticMeshComponent.SetStaticMesh` _arrow "/Game/Meshes/21325_Lightning_Bolt_v1.21325_Lightning_Bolt_v1")
            (`SceneComponent.K2_SetRelativeTransform` _arrow (`KismetMathLibrary.MakeTransform` (19.176498 19.19758 0.0) (struct :`Pitch` 70.0) (8.0 8.0 8.0)) false false)))
        (:`0`
          (`StaticMeshComponent.SetStaticMesh` _mesh_3 "/Game/Meshes/SM_CubeNote.SM_CubeNote")
          (`PrimitiveComponent.SetMaterial` _mesh_3 0 "/Game/Materials/M_CubeNote_red.M_CubeNote_red")
          (`PrimitiveComponent.SetMaterial` _arrow_2 0 "/Game/Materials/M_Arrow_red.M_Arrow_red")
          (if (== (`self.Direction`) 8) :!label _label
            (`StaticMeshComponent.SetStaticMesh` _arrow_3 "/Game/Meshes/SM_point.SM_point")
            (`SceneComponent.K2_SetRelativeLocation` _arrow_3 (0.0 25.0 0.0) false false)
            (else
              (`StaticMeshComponent.SetStaticMesh` _arrow_3 "/Game/Meshes/SM_Arrow.SM_Arrow")
              (`SceneComponent.K2_SetRelativeLocation` _arrow_3 (0.0 25.0 10.0) false false))))
        (:`1`
          (`StaticMeshComponent.SetStaticMesh` _mesh_3 "/Game/Meshes/SM_CubeNote.SM_CubeNote")
          (`PrimitiveComponent.SetMaterial` _mesh_3 0 "/Game/Materials/M_CubeNote_blue.M_CubeNote_blue")
          (`PrimitiveComponent.SetMaterial` _arrow_2 0 "/Game/Materials/M_Arrow_blue.M_Arrow_blue")
          (goto _label))
        (:`3`
          (`StaticMeshComponent.SetStaticMesh` _mesh_3 "/Game/Meshes/SM_Bomb.SM_Bomb")
          (`PrimitiveComponent.SetMaterial` _mesh_3 0 "/Game/Materials/M_bomb.M_bomb")
          (`SceneComponent.SetVisibility` (`self.Arrow`) false false))
        (:`4`
          (`StaticMeshComponent.SetStaticMesh` _mesh "/Game/Meshes/SM_CubeNote.SM_CubeNote")
          (`PrimitiveComponent.SetMaterial` _mesh 0 "/Game/Materials/M_CubeNote_mag.M_CubeNote_mag")
          (`PrimitiveComponent.SetMaterial` (`self.Arrow`) 0 "/Game/Materials/M_Arrow_mag.M_Arrow_mag")
          (goto _label))
        (:`5`
          (`StaticMeshComponent.SetStaticMesh` _mesh "/Game/Meshes/SM_CubeNote.SM_CubeNote")
          (`PrimitiveComponent.SetMaterial` _mesh 0 "/Game/Materials/M_CubeNote_green.M_CubeNote_green")
          (`PrimitiveComponent.SetMaterial` (`self.Arrow`) 0 "/Game/Materials/M_Arrow_green.M_Arrow_green")
          (goto _label))
        (:`6`
          (`StaticMeshComponent.SetStaticMesh` _mesh "/Game/Meshes/SM_CubeNote.SM_CubeNote")
          (`PrimitiveComponent.SetMaterial` _mesh 0 "/Game/Materials/M_CubeNote_grey.M_CubeNote_grey")
          (`PrimitiveComponent.SetMaterial` (`self.Arrow`) 0 "/Game/Materials/M_Arrow_grey.M_Arrow_grey")
          (goto _label))))
    (:`then_1`
      (`self.UpdateTransform`))))

(event `UpdateTransform`
  (`self.FixValues`)
  (`|ExecutionSequence`
    (:`then_0`
      (`SceneComponent.K2_SetRelativeRotation` (`self.Mesh`) (`KismetMathLibrary.MakeRotator` 0.0 (select `int` (`self.Direction`) :`0` 180.0 :`1` 0.0 :`2` 270.0 :`3` 90.0 :`4` 225.0 :`5` 135.0 :`6` 315.0 :`7` 45.0 :`8` 0.0 :`9` 0.0 :`10` 0.0 :!type "Float (single-precision)")) false false))
    (:`then_1`
      (`SceneComponent.K2_SetRelativeLocation` (`self.Mesh`) (`KismetMathLibrary.MakeVector` (- (* (`self.Line`) 70.0) 105.0) 0.0 (* (`self.Layer`) 70.0)) false false)
      (`self.K2_SetActorRelativeLocation` (`KismetMathLibrary.MakeVector` 0.0 (* (* (`/Game/Blueprints/BPFL_editor.GetNoteSep`) (`self.Time`)) -1.0))))))

(fn `FixValues`
  (bind _returnvalue (mod (`self.Layer`) 3))
  (bind _returnvalue_2 (mod (`self.Line`) 4))
  (set `self.Line` (select `bool` (< _returnvalue_2 0) :`false` _returnvalue_2 :`true` 3))
  (set `self.Layer` (select `bool` (< _returnvalue 0) :`false` _returnvalue :`true` 2)))

(fn `GetProperties`
  (returns (Note :type "/Game/Blueprints/VarTypes/StructNote Structure"))
  (return (make `/Game/Blueprints/VarTypes/StructNote` (`self.Time`) (`self.Line`) (`self.Layer`) (`self.Type`) (`self.Direction`))))

(fn `UserConstructionScript`
  (`self.Update Note`))